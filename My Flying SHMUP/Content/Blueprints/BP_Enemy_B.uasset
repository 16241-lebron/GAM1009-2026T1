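; BP_Enemy_B is an enemy Blueprint that periodically fires bullets.
; On BeginPlay it runs the parent logic, then starts a looping five-second timer that calls its shoot event.
; Each shot spawns a BP_EnemyFire_Bullet at the Arrow component's world location and rotation, so the arrow sets the muzzle point and firing direction.
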(event `self.ReceiveBeginPlay`
  (`parent.ReceiveBeginPlay`)
  (`KismetSystemLibrary.K2_SetTimerDelegate` (delegate `shoot bullet`) 5.0 true))

(event `shoot bullet`
  (bind _arrow (`self.Arrow`))
  (`|SpawnActorFromClass` "/Game/Blueprints/BP_EnemyFire_Bullet.BP_EnemyFire_Bullet_C" (`KismetMathLibrary.MakeTransform` (`SceneComponent.K2_GetComponentLocation` _arrow) (`SceneComponent.K2_GetComponentRotation` _arrow)) "Undefined" "MultiplyWithRoot" null null))

(fn `UserConstructionScript`
  (`parent.UserConstructionScript`))