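; BP_Projectile_Bullet3D is a bullet projectile Blueprint that sets its own movement speed when it spawns.
; On BeginPlay it runs the parent logic, sets ProjectileMovement's max and initial speed to Speed times Speedmultiplier, then activates the component.
; It adds no active overlap or tick logic, and its construction script only calls the parent.
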(event `self.ReceiveBeginPlay`
  (bind _projectilemovement (`self.ProjectileMovement`))
  (`parent.ReceiveBeginPlay`)
  (bind _output_get (set `ProjectileMovementComponent.MaxSpeed` (* (`self.speed`) (`self.speedmultiplier`)) _projectilemovement))
  (set `ProjectileMovementComponent.InitialSpeed` _output_get _projectilemovement)
  (`ActorComponent.Activate` _projectilemovement false))

(fn `UserConstructionScript`
  (`parent.UserConstructionScript`))