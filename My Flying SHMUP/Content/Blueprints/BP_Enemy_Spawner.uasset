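; Enemy spawner actor that periodically spawns a random enemy, either BP_Enemy_A or BP_Enemy_B, along a horizontal line.
; A looping timer started on BeginPlay drives each spawn.
; The LeftRange and RightRange components bound a random Y position, while X and rotation come from LeftRange and height is a fixed world Z.
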(event `self.ReceiveBeginPlay`
  (`KismetSystemLibrary.K2_SetTimerDelegate` (delegate `Spawn Enemy`) 3.0 true true))

(event `Spawn Enemy`
  (bind (_returnvalue_x _returnvalue_y) (`KismetMathLibrary.BreakVector` (`SceneComponent.K2_GetComponentLocation` (`self.Left Range`))))
  (bind (_returnvalue_x_2 _returnvalue_y_2) (`KismetMathLibrary.BreakVector` (`SceneComponent.K2_GetComponentLocation` (`self.Right Range`))))
  (`|SpawnActorFromClass` (`KismetArrayLibrary.Array_Random` (`|MakeArray` "/Game/Blueprints/BP_Enemy_A.BP_Enemy_A_C" "/Game/Blueprints/BP_Enemy_B.BP_Enemy_B_C" :!type "Actor Class Reference")) (`KismetMathLibrary.MakeTransform` (`KismetMathLibrary.MakeVector` _returnvalue_x (`KismetMathLibrary.RandomFloatInRange` (`KismetMathLibrary.FMin` _returnvalue_y _returnvalue_y_2) (`KismetMathLibrary.FMax` _returnvalue_y _returnvalue_y_2)) 400.0) (`SceneComponent.K2_GetComponentRotation` (`self.Left Range`))) "Undefined" "MultiplyWithRoot" null null))

(fn `UserConstructionScript`)