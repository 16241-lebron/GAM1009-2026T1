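; Boss enemy Blueprint that fires on a timer and ends the game with a win screen when killed.
; A looping timer fires from three arrow points along the mesh's rotation, though the third spawn has no class assigned.
; Damage lowers clamped Health, running a hit sequence or Death.
; Death plays an explosion sound, spawns an explosion, shows WinScreen and destroys the boss a frame later.
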(event `self.ReceiveAnyDamage`
  (params (Damage :type "Float (single-precision)") (DamageType :type "DamageType Object Reference") (InstigatedBy :type "Controller Object Reference") (DamageCauser :type "Actor Object Reference"))
  (bind _output_get (set `self.Health` (`KismetMathLibrary.FMax` (- (`self.Health`) Damage))))
  (if (<= _output_get 0.0)
    (`self.death`)
    (else
      (`self.Hitsequence`))))

(event `self.death`
  (`|ExecutionSequence`
    (:`then_0`
      (`GameplayStatics.PlaySound2D` "/Game/Audios/Retro_Explosion_Short_01.Retro_Explosion_Short_01" 0.5 1.0 0.0 null null))
    (:`then_1`
      (`|SpawnActorFromClass` "/Game/Particles/BP_Explosion.BP_Explosion_C" (`KismetMathLibrary.MakeTransform` (`self.K2_GetActorLocation`)) "Undefined" "MultiplyWithRoot" null null))
    (:`then_2`
      (bind _returnvalue (`|CreateWidget` "/Game/UI/WinScreen.WinScreen_C"))
      (`UserWidget.AddToViewport` _returnvalue 0))
    (:`then_3`
      (`KismetSystemLibrary.DelayUntilNextFrame`)
      (`self.K2_DestroyActor`))))

(event `self.ReceiveBeginPlay`
  (`parent.ReceiveBeginPlay`)
  (`KismetSystemLibrary.K2_SetTimerDelegate` (delegate `shoot bullet`) 1.0 true))

(event `shoot bullet`
  (`|SpawnActorFromClass` "/Game/Blueprints/BP_EnemyFire_Bullet.BP_EnemyFire_Bullet_C" (`KismetMathLibrary.MakeTransform` (`SceneComponent.K2_GetComponentLocation` (`self.Arrow`)) (`SceneComponent.K2_GetComponentRotation` (`self.Mesh`))) "Undefined" "MultiplyWithRoot" null null)
  (`|SpawnActorFromClass` "/Game/Blueprints/BP_EnemyFire_Bullet.BP_EnemyFire_Bullet_C" (`KismetMathLibrary.MakeTransform` (`SceneComponent.K2_GetComponentLocation` (`self.Arrow1`)) (`SceneComponent.K2_GetComponentRotation` (`self.Mesh`))) "Undefined" "MultiplyWithRoot" null null)
  (`|SpawnActorFromClass` "/Game/Blueprints/BP_EnemyFire_Bullet.BP_EnemyFire_Bullet_C" (`KismetMathLibrary.MakeTransform` (`SceneComponent.K2_GetComponentLocation` (`self.Arrow2`)) (`SceneComponent.K2_GetComponentRotation` (`self.Mesh`))) "Undefined" "MultiplyWithRoot" null null))

(event `self.ReceiveTick`
  (params (DeltaSeconds :type "Float (single-precision)"))
  (`parent.ReceiveTick` 0.0))

(fn `UserConstructionScript`
  (`parent.UserConstructionScript`))