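; BP_Enemy_Spawner_InZone is a zone spawner that keeps creating enemies inside a box area.
; The construction script sizes the box from BoxExtent.
; A looping one-second timer starts at BeginPlay and calls SpawnEnemy, which has no count limit.
; Each spawn uses a random stream to pick from a class array holding only BP_Enemy_D and X/Y within the box, with rotation from the Arrow and Z left unset.
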(event `self.ReceiveBeginPlay`
  (`KismetSystemLibrary.K2_SetTimerDelegate` (delegate `Spawn Enemy`) 1.0 true true))

(event `Spawn Enemy`
  (bind _box (`self.Box`))
  (bind _stream (`self.Stream`))
  (bind (_returnvalue_x _returnvalue_y) (`KismetMathLibrary.BreakVector` (`KismetMathLibrary.RandomPointInBoundingBoxFromStream` _stream (`SceneComponent.K2_GetComponentLocation` _box) (`BoxComponent.GetScaledBoxExtent` _box))))
  (`|SpawnActorFromClass` (`KismetArrayLibrary.Array_RandomFromStream` (`|MakeArray` "/Game/Blueprints/BP_Enemy_D.BP_Enemy_D_C" :!type "Actor Class Reference") _stream) (`KismetMathLibrary.MakeTransform` (`KismetMathLibrary.MakeVector` _returnvalue_x _returnvalue_y) (`SceneComponent.K2_GetComponentRotation` (`self.Arrow`))) "Undefined" "MultiplyWithRoot" null null))

(fn `UserConstructionScript`
  (`BoxComponent.SetBoxExtent` (`self.Box`) (`self.BoxExtent`) false))