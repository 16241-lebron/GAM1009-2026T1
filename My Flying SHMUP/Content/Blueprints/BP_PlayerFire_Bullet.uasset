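; BP_PlayerFire_Bullet is a projectile Blueprint for the bullets the player fires.
; On BeginPlay it sets the ProjectileMovement max and initial speed from Speed times Speedmultiplier, then activates the component.
; It then plays the player shoot sound as a non-spatial 2D sound.
; The graph holds no hit or overlap logic of its own, only calls to the parent.
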(event `self.ReceiveBeginPlay`
  (bind _projectilemovement (`self.ProjectileMovement`))
  (`parent.ReceiveBeginPlay`)
  (`|ExecutionSequence`
    (:`then_0`
      (bind _output_get (set `ProjectileMovementComponent.MaxSpeed` (* (`self.speed`) (`self.speedmultiplier`)) _projectilemovement))
      (set `ProjectileMovementComponent.InitialSpeed` _output_get _projectilemovement)
      (`ActorComponent.Activate` _projectilemovement false))
    (:`then_1`
      (`GameplayStatics.PlaySound2D` "/Game/Audios/shoot_sound_player.shoot_sound_player" 1.0 1.0 0.0 null null))))

(fn `UserConstructionScript`
  (`parent.UserConstructionScript`))