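; Wave 5 enemy spawner that brings the boss enemy BP_Enemy_E_Boss into the level after a long delay.
; BeginPlay sets a non-looping timer, delayed by over a minute, that fires SpawnEnemy.
; SpawnEnemy places the boss at the horizontal midpoint of the LeftRange and RightRange components, at a fixed world height, using LeftRange's rotation.
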(event `self.ReceiveBeginPlay`
  (`KismetSystemLibrary.K2_SetTimerDelegate` (delegate `Spawn Enemy`) 1.0 false true 75.0))

(event `Spawn Enemy`
  (bind (_returnvalue_x _returnvalue_y) (`KismetMathLibrary.BreakVector` (`KismetMathLibrary.VLerp` (`SceneComponent.K2_GetComponentLocation` (`self.Left Range`)) (`SceneComponent.K2_GetComponentLocation` (`self.Right Range`)) 0.5)))
  (`|SpawnActorFromClass` "/Game/Blueprints/BP_Enemy_E_Boss.BP_Enemy_E_Boss_C" (`KismetMathLibrary.MakeTransform` (`KismetMathLibrary.MakeVector` _returnvalue_x _returnvalue_y 400.0) (`SceneComponent.K2_GetComponentRotation` (`self.Left Range`))) "Undefined" "MultiplyWithRoot" null null))

(fn `UserConstructionScript`)