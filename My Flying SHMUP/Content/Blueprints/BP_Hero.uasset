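; Player hero pawn for a flying shoot 'em up that moves, fires, damages actors it overlaps and shakes the camera when hit.
; On possession it caches the player controller and adds the Enhanced Input context, whose move actions drive FloatingPawnMovement.
; Primary fire reads weapon settings from that controller, using nested loops for staggered, spread bullet spawns and a DoOnce reset by fire rate.
; Only shooting mode 0 is implemented.
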(event `self.ReceiveActorBeginOverlap`
  (params (OtherActor :type "Actor Object Reference"))
  (`GameplayStatics.ApplyDamage` OtherActor (`self.body slam damage`)))

(event `self.ReceivePossessed`
  (params (NewController :type "Controller Object Reference"))
  ; Adds input mapping context for the owning controller if it is a player controller
  (bind _asplayer_controller_my_flying_shmup (cast `/Game/Core/PlayerController_MyFlyingSHMUP` NewController))
  (set `self.AsPlayer Controller My Flying SHMUP` _asplayer_controller_my_flying_shmup)
  (`EnhancedInputSubsystemInterface.AddMappingContext` (pcsubsystem `EnhancedInputLocalPlayerSubsystem` _asplayer_controller_my_flying_shmup) "/Game/Inputs/IMC_Hero.IMC_Hero" 0 (struct)))

(event `EnhancedInput|/Game/Inputs/IA_MoveForwardBackwards`
  (params (ActionValue :type "Float (double-precision)") (ElapsedSeconds :type "Float (double-precision)") (TriggeredSeconds :type "Float (double-precision)") (InputAction :type "InputAction Object Reference" :default "/Game/Inputs/IA_MoveForwardBackwards.IA_MoveForwardBackwards"))
  ; Movement
  (:`Triggered`
    (`PawnMovementComponent.AddInputVector` (`self.FloatingPawnMovement`) (`KismetMathLibrary.MakeVector` ActionValue) false)))

(event `self.ReceiveAnyDamage`
  (params (Damage :type "Float (single-precision)") (DamageType :type "DamageType Object Reference") (InstigatedBy :type "Controller Object Reference") (DamageCauser :type "Actor Object Reference"))
  (`PlayerController.ClientStartCameraShake` :`self` (`GameplayStatics.GetPlayerController` 0) :`Shake` "/Game/Blueprints/BP_CameraShake.BP_CameraShake_C"))

(event `EnhancedInput|/Game/Inputs/IA_MoveRightLeft`
  (params (ActionValue :type "Float (double-precision)") (ElapsedSeconds :type "Float (double-precision)") (TriggeredSeconds :type "Float (double-precision)") (InputAction :type "InputAction Object Reference" :default "/Game/Inputs/IA_MoveRightLeft.IA_MoveRightLeft"))
  ; Movement
  (:`Triggered`
    (`PawnMovementComponent.AddInputVector` (`self.FloatingPawnMovement`) (`KismetMathLibrary.MakeVector` 0.0 ActionValue) false)))

(event `EnhancedInput|/Game/Inputs/IA_PrimaryFire`
  (params (ActionValue :type Boolean) (ElapsedSeconds :type "Float (double-precision)") (TriggeredSeconds :type "Float (double-precision)") (InputAction :type "InputAction Object Reference" :default "/Game/Inputs/IA_PrimaryFire.IA_PrimaryFire"))
  (:`Triggered`
    (bind _asplayer_controller_my_flying_shmup (`self.AsPlayer Controller My Flying SHMUP`)
      (:`then`
        (set `self.Shooting mode` (`/Game/Core/PlayerController_MyFlyingSHMUP.Shooting mode` _asplayer_controller_my_flying_shmup))
        (set `self.simulbulletstoshoot` (`/Game/Core/PlayerController_MyFlyingSHMUP.simulbulletstoshoot` _asplayer_controller_my_flying_shmup))
        (set `self.shooting direction` (`/Game/Core/PlayerController_MyFlyingSHMUP.shooting direction` _asplayer_controller_my_flying_shmup))
        (set `self.rate of fire` (`/Game/Core/PlayerController_MyFlyingSHMUP.rate of fire` _asplayer_controller_my_flying_shmup))
        (switch `int` (`self.Shooting mode`)
          (:`0`
            (`/Engine/EditorBlueprintResources/StandardMacros.DoOnce` false :!label _label
              (:`Completed`
                (`|ExecutionSequence`
                  (:`then_0`
                    (for _index (range (+ (`self.simulbulletstoshoot`) 1))
                      (switch `int` _index
                        (:`0`
                          _)
                        (:`1`
                          (`KismetSystemLibrary.Delay` 0.1))
                        (:`2`
                          (`KismetSystemLibrary.Delay` 0.2)))
                      (for _index_2 (range (+ (`self.shooting direction`) 1))
                        (switch `int` _index_2
                          (:`0`
                            (`self.Fire single bullet` (0.0 0.0 0.0) :!label _label_2))
                          (:`1`
                            (`self.Fire single bullet` (0.0 100.0 0.0))
                            (`self.Fire single bullet` (0.0 -100.0 0.0)))
                          (:`2`
                            (`self.Fire single bullet` (-200.0 200.0 0.0) 10.0)
                            (`self.Fire single bullet` (-200.0 -200.0 0.0) -10.0)
                            (goto _label_2))))))
                  (:`then_1`
                    (`KismetSystemLibrary.Delay` (`self.rate of fire`))
                    (goto _label :!via `Reset`))))))))
      (:`else`))))

(event `Fire single bullet`
  (params (`Relative Location` :type "Vector Structure") (`Relative Angle` :type "Float (double-precision)"))
  (`|SpawnActorFromClass` "/Game/Blueprints/BP_PlayerFire_Bullet.BP_PlayerFire_Bullet_C" (`KismetMathLibrary.MakeTransform` (+ `Relative Location` (`SceneComponent.K2_GetComponentLocation` (`self.Bullet Spawn`))) (`KismetMathLibrary.MakeRotator` 0.0 0.0 `Relative Angle`)) "AlwaysSpawn" "MultiplyWithRoot" (`self.GetLocalViewingPlayerController`) 8000.0 1.0 self))

(fn `UserConstructionScript`)