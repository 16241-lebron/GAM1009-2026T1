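; Player-possessed helicopter-style pawn that flies with Enhanced Input and fires bullet projectiles from an Arrow component after a short delay.
; FloatingPawnMovement handles forward/back and vertical motion, while left/right input yaws the whole actor.
; Tick eases cosmetic roll on Body and pitch on the Pitch component toward input-scaled limits using FInterpTo.
; RotatingMovement spins the main rotor, switching to a faster rate while ascending.
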(event `self.ReceivePossessed`
  (params (NewController :type "Controller Object Reference"))
  (bind _asplayer_controller (cast `PlayerController` NewController))
  (`EnhancedInputSubsystemInterface.AddMappingContext` (pcsubsystem `EnhancedInputLocalPlayerSubsystem` _asplayer_controller) "/Game/Inputs/IMC_ADVANCED.IMC_ADVANCED" 0 (struct)))

(event `self.ReceiveBeginPlay`
  (`MovementComponent.SetUpdatedComponent` (`self.RotatingMovement`) (`self.MainRotor`)))

(event `EnhancedInput|/Game/Inputs/IA_PrimaryFire`
  (params (ActionValue :type Boolean) (ElapsedSeconds :type "Float (double-precision)") (TriggeredSeconds :type "Float (double-precision)") (InputAction :type "InputAction Object Reference" :default "/Game/Inputs/IA_PrimaryFire.IA_PrimaryFire"))
  (bind _arrow (`self.Arrow`))
  (:`Triggered`
    (`KismetSystemLibrary.Delay` 0.2)
    (`|SpawnActorFromClass` "/Game/Blueprints/BP_Projectile_Bullet.BP_Projectile_Bullet_C" (`KismetMathLibrary.MakeTransform` (`SceneComponent.K2_GetComponentLocation` _arrow) (`SceneComponent.K2_GetComponentRotation` _arrow)) "AlwaysSpawn" "MultiplyWithRoot" (`self.GetLocalViewingPlayerController`) self)))

(event `EnhancedInput|/Game/Inputs/IA_MoveForwardBackwards`
  (params (ActionValue :type "Float (double-precision)") (ElapsedSeconds :type "Float (double-precision)") (TriggeredSeconds :type "Float (double-precision)") (InputAction :type "InputAction Object Reference" :default "/Game/Inputs/IA_MoveForwardBackwards.IA_MoveForwardBackwards"))
  (:`Triggered`
    (`PawnMovementComponent.AddInputVector` (`self.FloatingPawnMovement`) (* (`self.GetActorForwardVector`) ActionValue) false)))

(event `EnhancedInput|/Game/Inputs/IA_MoveUpDown`
  (params (ActionValue :type "Float (double-precision)") (ElapsedSeconds :type "Float (double-precision)") (TriggeredSeconds :type "Float (double-precision)") (InputAction :type "InputAction Object Reference" :default "/Game/Inputs/IA_MoveUpDown.IA_MoveUpDown"))
  (:`Triggered`
    (`PawnMovementComponent.AddInputVector` (`self.FloatingPawnMovement`) (`KismetMathLibrary.MakeVector` 0.0 0.0 ActionValue) false)))

(event `EnhancedInput|/Game/Inputs/IA_MoveRightLeft`
  (params (ActionValue :type "Float (double-precision)") (ElapsedSeconds :type "Float (double-precision)") (TriggeredSeconds :type "Float (double-precision)") (InputAction :type "InputAction Object Reference" :default "/Game/Inputs/IA_MoveRightLeft.IA_MoveRightLeft"))
  (:`Triggered`
    (`self.K2_AddActorLocalRotation` (`KismetMathLibrary.MakeRotator` 0.0 0.0 ActionValue))))

(event `self.ReceiveTick`
  (params (DeltaSeconds :type "Float (single-precision)"))
  (set `self.DeltaSeconds` DeltaSeconds)
  (`|ExecutionSequence`
    (:`then_0`
      (set `self.TargetRollAngle` (* (`|GetInputActionValue`) (`self.MaxRollAngle`)))
      (bind _output_get (set `self.CurrentRollAngle` (`KismetMathLibrary.FInterpTo` (`self.CurrentRollAngle`) (`self.TargetRollAngle`) (`self.DeltaSeconds`) 4.0)))
      (`SceneComponent.K2_SetRelativeRotation` (`self.Body`) (`KismetMathLibrary.MakeRotator` _output_get) false false))
    (:`then_1`
      (bind _output_get_2 (set `self.IsMovingUp` (> (`|GetInputActionValue`) 0.0)))
      (if _output_get_2
        (set `RotatingMovementComponent.RotationRate` (`KismetMathLibrary.MakeRotator` 0.0 0.0 1280.0) (`self.RotatingMovement`))
        (else
          (set `RotatingMovementComponent.RotationRate` (`KismetMathLibrary.MakeRotator` 0.0 0.0 720.0) (`self.RotatingMovement`)))))
    (:`then_2`
      (set `self.TargetPitchAngle` (* (`|GetInputActionValue`) (`self.MaxPitchAngle`) -1.0))
      (bind _output_get_3 (set `self.CurrentPitchAngle` (`KismetMathLibrary.FInterpTo` (`self.CurrentPitchAngle`) (`self.TargetPitchAngle`) (`self.DeltaSeconds`) 4.0)))
      (`SceneComponent.K2_SetRelativeRotation` (`self.Pitch`) (`KismetMathLibrary.MakeRotator` 0.0 _output_get_3) false false))))

(fn `UserConstructionScript`)