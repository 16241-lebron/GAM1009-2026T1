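; Enemy actor that turns to face the player and periodically fires BP_EnemyFire_Bullet projectiles.
; Tick yaws the mesh toward the first player's pawn using a look-at rotation.
; A looping timer started on BeginPlay spawns each bullet at the actor's location with the mesh's yaw.
; BeginPlay also caches the WBP_EnemyHealthBar from its widget component, though this graph never updates it.
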(event `self.ReceiveBeginPlay`
  (`|ExecutionSequence`
    (:`then_0`
      (bind _aswbp_enemy_health_bar (cast `/Game/UI/WBP_EnemyHealthBar` (`WidgetComponent.GetUserWidgetObject` (`self.Widget`))))
      (set `self.Healthbar` _aswbp_enemy_health_bar))
    (:`then_1`
      (`KismetSystemLibrary.K2_SetTimerDelegate` (delegate `Shoot bullet`) 3.0 true))))

(event `Shoot bullet`
  (bind (_returnvalue_roll _returnvalue_pitch _returnvalue_yaw) (`KismetMathLibrary.BreakRotator` (`SceneComponent.K2_GetComponentRotation` (`self.Mesh`))))
  (`|SpawnActorFromClass` "/Game/Blueprints/BP_EnemyFire_Bullet.BP_EnemyFire_Bullet_C" (`KismetMathLibrary.MakeTransform` (`self.K2_GetActorLocation`) (`KismetMathLibrary.MakeRotator` 0.0 0.0 _returnvalue_yaw)) "Undefined" "MultiplyWithRoot" null null))

(event `self.ReceiveTick`
  (params (DeltaSeconds :type "Float (single-precision)"))
  (bind (_returnvalue_roll _returnvalue_pitch _returnvalue_yaw) (`KismetMathLibrary.BreakRotator` (`KismetMathLibrary.FindLookAtRotation` (`self.K2_GetActorLocation`) (`self.K2_GetActorLocation` (`GameplayStatics.GetPlayerPawn` 0)))))
  (`SceneComponent.K2_SetWorldRotation` (`self.Mesh`) (`KismetMathLibrary.MakeRotator` 0.0 0.0 _returnvalue_yaw) false false))

(fn `UserConstructionScript`
  (`parent.UserConstructionScript`))