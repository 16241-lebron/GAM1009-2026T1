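; Enemy spawner actor, named for wave 3, that spawns BP_Enemy inside a configurable box area.
; BeginPlay starts a looping half-second timer after a 40-second delay, stopping once SpawnCount reaches MaxSpawnCount.
; Each spawn takes random X and Y from the box using a random stream, with rotation from the Arrow component.
; The construction script sizes the box from BoxExtent.
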(event `self.ReceiveBeginPlay`
  (bind _returnvalue (`KismetSystemLibrary.K2_SetTimerDelegate` (delegate `Spawn Enemy`) 0.5 true false 40.0))
  (set `self.Timer` _returnvalue))

(event `Spawn Enemy`
  (bind _box (`self.Box`))
  (bind _stream (`self.Stream`))
  (bind (_returnvalue_x _returnvalue_y) (`KismetMathLibrary.BreakVector` (`KismetMathLibrary.RandomPointInBoundingBoxFromStream` _stream (`SceneComponent.K2_GetComponentLocation` _box) (`BoxComponent.GetScaledBoxExtent` _box))))
  (`|SpawnActorFromClass` (`KismetArrayLibrary.Array_RandomFromStream` (`|MakeArray` "/Game/Blueprints/BP_Enemy_C.BP_Enemy_C_C" :!type "Actor Class Reference") _stream) (`KismetMathLibrary.MakeTransform` (`KismetMathLibrary.MakeVector` _returnvalue_x _returnvalue_y) (`SceneComponent.K2_GetComponentRotation` (`self.Arrow`))) "Undefined" "MultiplyWithRoot" null null)
  (set `self.Spawn Count` (+ (`self.Spawn Count`) 1))
  (if (>= (`self.Spawn Count`) (`self.Max Spawn Count`))
    (`KismetSystemLibrary.K2_ClearAndInvalidateTimerHandle` (`self.Timer`))))

(fn `UserConstructionScript`
  (`BoxComponent.SetBoxExtent` (`self.Box`) (`self.BoxExtent`) false))